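; Stage director that populates stages with upgrade pedestals and responds to stage and tavern transitions from the Megadeth stage subsystem.
; On stage entry, including at BeginPlay, it updates difficulty, then spends EnemyCredits spawning tagged pedestals at random navigable points, each assigned a random data table upgrade.
; On tavern entry it updates difficulty and sets the tagged tavern portal's level location to a random navigable point.
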(event `self.ReceiveBeginPlay`
  (bind _returnvalue (subsystem `MegadethStageSubsystem`))
  (`|ExecutionSequence`
    (:`then_0`
      (add `MegadethStageSubsystem.EnteredStage` _returnvalue (delegate `EnteredStage`))
      (`self.EnteredStage`))
    (:`then_1`
      (add `MegadethStageSubsystem.EnteredTavern` _returnvalue (delegate `EnteredTavern`)))))

(event `EnteredStage`
  (bind _output (`|ConvertAsset` (`self.InteractableTable`)))
  (`self.UpdateDifficulty`)
  (`|ExecutionSequence`
    (:`then_0`
      (while (> (`self.EnemyCredits`) 0.0)
        (bind (_randomlocation _returnvalue) (`NavigationSystemV1.K2_GetRandomLocationInNavigableRadius` (`KismetMathLibrary.RandomPointInBoundingBox` (0.0 0.0 0.0) (3000.0 3000.0 3000.0)) 3000.0 null null))
        (if _returnvalue
          (bind _returnvalue_2 (`|SpawnActorFromClass` (`|ConvertAsset` (`self.InteractableClass`)) (`KismetMathLibrary.MakeTransform` _randomlocation) "Undefined" "MultiplyWithRoot" null null))
          (bind _asbp_upgrade_pedestal (cast `/Game/Blueprints/BP_UpgradePedestal` _returnvalue_2))
          (set `Actor.Tags` (`|MakeArray` "FieldUpgradePickup") _asbp_upgrade_pedestal)
          (set `self.EnemyCredits` (- (`self.EnemyCredits`) (`self.InteractableCost`)))
          (bind _outrownames (`DataTableFunctionLibrary.GetDataTableRowNames` _output))
          (bind _returnvalue_3 (`|GetDataTableRow` _output (`KismetArrayLibrary.Array_Random` _outrownames))
            (:`then`
              (set `/Game/Blueprints/BP_UpgradePedestal.UpgradeToAdd` (`.Upgrade_4_249BC6254C4F60D313D42F80509374D4` (break `/Game/Structs/F_UpgradeRoulletteList` _returnvalue_3)) _asbp_upgrade_pedestal))))))))

(event `EnteredTavern`
  (`self.UpdateDifficulty`)
  (bind _randomlocation (`NavigationSystemV1.K2_GetRandomLocationInNavigableRadius` (`KismetMathLibrary.RandomPointInBoundingBox` (0.0 0.0 0.0) (3000.0 3000.0 3000.0)) 3000.0 null null))
  (bind _outactors (`GameplayStatics.GetAllActorsWithTag` "TavernPortal"))
  (bind _asbp_tavern_portal (cast `/Game/Blueprints/BP_TavernPortal` (`|GetArrayItem` _outactors)))
  (set `/Game/Blueprints/BP_TavernPortal.LevelLocation` _randomlocation _asbp_tavern_portal))

(fn `UserConstructionScript`)