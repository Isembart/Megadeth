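; BP_SkillPickup is a world pickup that lets the MegadethCharacter replace one of its skills, showing that skill's splash art on its sphere.
; On overlap it disables input, spawns the skill actor and passes it to a W_SkillOverrideScreen widget.
; Selecting a slot writes the skill class into the character's Skills array and notifies MegadethAbilityExchangeSubsystem.
; Selecting or discarding removes the widget, restores input and destroys the pickup.
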(event `self.ReceiveBeginPlay`
  (bind _returnvalue (`PrimitiveComponent.CreateDynamicMaterialInstance` (`self.Sphere`) 0 "/Game/NewMaterial.NewMaterial" "None"))
  (`MaterialInstanceDynamic.SetTextureParameterValue` _returnvalue "Texture" (`.AbilitySplashArt` (break `MegadethAbilityData` (defaults `Object` (`self.SkillToAdd`))))))

(event `self.ReceiveActorBeginOverlap`
  (params (OtherActor :type "Actor Object Reference"))
  (bind _skill_override_screen_widget (`self.Skill Override Screen Widget`))
  (bind _asmegadeth_character (cast `MegadethCharacter` OtherActor))
  (set `self.PlayerMegadethCharacter` _asmegadeth_character)
  (`self.DisableInput` (`GameplayStatics.GetPlayerController` 0) null)
  (bind _returnvalue (`|SpawnActorFromClass` (`self.SkillToAdd`) (`KismetMathLibrary.MakeTransform` (0.0 0.0 0.0)) "Undefined" "MultiplyWithRoot" null null))
  (bind _returnvalue_2 (`|CreateWidget` "/Game/UI/W_SkillOverrideScreen.W_SkillOverrideScreen_C" null _returnvalue))
  (bind _output_get (set `self.Skill Override Screen Widget` _returnvalue_2))
  (`UserWidget.AddToViewport` _output_get 0)
  (`|ExecutionSequence`
    (:`then_0`
      (add `/Game/UI/W_SkillOverrideScreen.SkillSelected` _skill_override_screen_widget (delegate `Skill Selected`)))
    (:`then_1`
      (add `/Game/UI/W_SkillOverrideScreen.SkillDiscarded` _skill_override_screen_widget (delegate `Skill Discarded`)))))

(event `Skill Discarded`
  (`self.ClearWidgetAndEnableMovement`))

(event `Skill Selected`
  (params (SkillIndex :type Integer))
  (`KismetArrayLibrary.Array_Set` (`MegadethCharacter.Skills` (`self.PlayerMegadethCharacter`)) SkillIndex (`self.SkillToAdd`))
  (`MegadethAbilityExchangeSubsystem.ExchangedSkills` (subsystem `MegadethAbilityExchangeSubsystem`))
  (`self.ClearWidgetAndEnableMovement`))

(fn `ClearWidgetAndEnableMovement`
  (`Widget.RemoveFromParent` (`self.Skill Override Screen Widget`))
  (`self.EnableInput` (`GameplayStatics.GetPlayerController` 0) null)
  (`self.K2_DestroyActor`))

(fn `UserConstructionScript`)