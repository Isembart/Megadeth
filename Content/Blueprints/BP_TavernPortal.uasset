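; Two-way teleport portal between the stage and the streamed Tavern level, with the TavernPortal tag marking the tavern-side instance.
; A stage portal loads Tavern, finds its counterpart by tag, and scales over a Decay timeline until destroyed.
; Entering it teleports the MegadethCharacter there, enabling the return collision after a delay to avoid bouncing back.
; The tavern portal returns players to LevelLocation and unloads Tavern; both directions notify MegadethStageSubsystem.
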(event `self.ReceiveBeginPlay`
  (set `PrimitiveComponent.bGenerateOverlapEvents` false (`self.SphereCollision`))
  (bind _output_get (set `self.AtTavern` (`self.ActorHasTag` "TavernPortal")))
  (if (not _output_get)
    (`GameplayStatics.LoadStreamLevel` "Tavern" true)
    (set `PrimitiveComponent.bGenerateOverlapEvents` true (`self.Sphere`))
    (bind _outactors (`GameplayStatics.GetAllActorsWithTag` "TavernPortal"))
    (bind _asbp_tavern_portal (cast `/Game/Blueprints/BP_TavernPortal` (`|GetArrayItem` _outactors)))
    (set `self.PortalAtTavern` _asbp_tavern_portal)
    (bind (_direction _sizemultiplier) (`Timeline|Decay`)
      (:`Update`
        (`SceneComponent.SetRelativeScale3D` (`self.Sphere`) (* (5.0 4.0 2.0) _sizemultiplier)))
      (:`Finished`
        (`self.K2_DestroyActor`)))))

(event `self.ReceiveActorBeginOverlap`
  (params (OtherActor :type "Actor Object Reference"))
  (bind _portalattavern (`self.PortalAtTavern`))
  (bind _asmegadeth_character (cast `MegadethCharacter` OtherActor))
  (if (`self.AtTavern`)
    (`self.K2_TeleportTo` :`self` _asmegadeth_character :`DestLocation` (`self.LevelLocation`))
    (`MegadethStageSubsystem.OnEnteredStage` (subsystem `MegadethStageSubsystem`))
    (`GameplayStatics.UnloadStreamLevel` "Tavern")
    (else
      (set `PrimitiveComponent.bGenerateOverlapEvents` false (`/Game/Blueprints/BP_TavernPortal.Sphere` _portalattavern))
      (`self.K2_TeleportTo` :`self` _asmegadeth_character :`DestLocation` (`self.K2_GetActorLocation` _portalattavern))
      (`MovementComponent.StopMovementImmediately` (`Character.CharacterMovement` _asmegadeth_character))
      (`KismetSystemLibrary.Delay` 2.0)
      (set `PrimitiveComponent.bGenerateOverlapEvents` true (`/Game/Blueprints/BP_TavernPortal.SphereCollision` (`self.PortalAtTavern`)))
      (`MegadethStageSubsystem.OnEnteredTavern` (subsystem `MegadethStageSubsystem`))
      (`self.K2_DestroyActor`))))

(fn `UserConstructionScript`)