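; BP_Bullet is a projectile actor that damages BP_Enemy actors it overlaps.
; Tick moves it along its forward vector at a fixed speed without sweeping, and BeginPlay destroys it after a short delay.
; On overlapping an enemy it applies its Damage value and destroys itself, ignoring all other actors.
; A disconnected chain that would spawn a damage pop-up showing that value never runs.
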(event `self.ReceiveBeginPlay`
  (`KismetSystemLibrary.Delay` 5.0)
  (`self.K2_DestroyActor`))

(event `self.ReceiveTick`
  (params (DeltaSeconds :type "Float (single-precision)"))
  (`self.K2_AddActorWorldOffset` (* (`self.GetActorForwardVector`) (`KismetMathLibrary.Conv_DoubleToVector` 5000.0) DeltaSeconds)))

(event `self.ReceiveActorBeginOverlap`
  (params (OtherActor :type "Actor Object Reference"))
  (bind _asbp_enemy (cast `/Game/Blueprints/Enemies/BP_Enemy` OtherActor))
  (`GameplayStatics.ApplyDamage` _asbp_enemy (`self.Damage`))
  (`self.K2_DestroyActor`))

(fn `UserConstructionScript`)