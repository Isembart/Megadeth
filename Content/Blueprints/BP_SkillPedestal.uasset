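; BP_SkillPedestal is an interactable pedestal that offers a random skill and displays a cost.
; On BeginPlay it picks a skill from a data table, shows Cost as text and puts the skill's splash art on the orb through a dynamic material.
; Interacting spawns a BP_SkillPickup carrying that skill beside the pedestal, with no cost check in this graph.
; Tick yaws the text toward the player.
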(event `self.ReceiveBeginPlay`
  (`parent.ReceiveBeginPlay`)
  (add `self.InteractDelegate` (delegate `interactEvent`))
  (bind _outrownames (`DataTableFunctionLibrary.GetDataTableRowNames` (`self.SkillsDataTable`)))
  (bind _returnvalue (`|GetDataTableRow` (`self.SkillsDataTable`) (`KismetArrayLibrary.Array_Random` _outrownames))
    (:`then`
      (set `self.SkillToAdd` (`.Ability_2_249BC6254C4F60D313D42F80509374D4` (break `/Game/Structs/F_AbilityRoulletteListItem` _returnvalue)))
      (`TextRenderComponent.K2_SetText` (`self.SkillName`) (`KismetTextLibrary.Conv_IntToText` (`self.Cost`)))
      (bind _returnvalue_2 (`PrimitiveComponent.CreateDynamicMaterialInstance` (`self.Sphere_0`) 0 "/Game/Materials/M_PickupOrbMaterial.M_PickupOrbMaterial" "None"))
      (`MaterialInstanceDynamic.SetTextureParameterValue` _returnvalue_2 "Texture" (`.AbilitySplashArt` (break `MegadethAbilityData` (defaults `Object` (`self.SkillToAdd`))))))
    (:`RowNotFound`
      (`KismetSystemLibrary.PrintString` "BP_SkillPedestal ddn't find suitable skill in it's data table!"))))

(event `interactEvent` :!signature `self.InteractDelegate`
  (params (`Character To Interact` :type "MegadethCharacter Object Reference"))
  (`self.OnInteracted` `Character To Interact`))

(event `self.ReceiveTick`
  (params (DeltaSeconds :type "Float (single-precision)"))
  (bind _skillname (`self.SkillName`))
  (`parent.ReceiveTick` DeltaSeconds)
  (`SceneComponent.K2_SetWorldRotation` _skillname (`KismetMathLibrary.MakeRotator` 0.0 0.0 (.yaw (.rotation (`KismetAnimationLibrary.K2_LookAt` (`SceneComponent.K2_GetComponentToWorld` _skillname) (`self.K2_GetActorLocation` (`GameplayStatics.GetPlayerPawn` 0)) (1.0 0.0 0.0))))) false false))

(fn `OnInteracted`
  (params (Character :type "MegadethCharacter Object Reference"))
  (bind _returnvalue_location (`KismetMathLibrary.BreakTransform` (`self.GetTransform`)))
  (`|SpawnActorFromClass` "/Game/Blueprints/BP_SkillPickup.BP_SkillPickup_C" (`KismetMathLibrary.MakeTransform` (+ _returnvalue_location (-100.0 100.0 0.0))) "Undefined" "MultiplyWithRoot" null (`self.SkillToAdd`) null))

(fn `UserConstructionScript`)