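; BP_DamageUp is an upgrade that raises the equipping character's base damage by five percent.
; On BeginPlay it binds OnEquipped to the equipped dispatcher.
; When equipped, it multiplies BaseDamage in the character's MegadethPlayerStats struct, writes the struct back, then calls AddXp with zero, granting no experience.
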(event `self.ReceiveBeginPlay`
  (add `self.EquippedDispatcher` (delegate `OnEquipped`))
  (`parent.ReceiveBeginPlay`))

(event `OnEquipped` :!signature `self.EquippedDispatcher`
  (params (Character :type "MegadethCharacter Object Reference"))
  (bind _stats (`MegadethCharacter.Stats` Character))
  (bind _structout (setmembers `MegadethPlayerStats` :`StructRef` _stats :`BaseDamage` (* (`.BaseDamage` (break `MegadethPlayerStats` _stats)) 1.05)))
  (set `MegadethCharacter.Stats` _structout Character)
  (`MegadethCharacter.AddXp` Character 0))