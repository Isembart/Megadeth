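; BP_HealthRegen is an upgrade that boosts a character's health regeneration when equipped.
; On BeginPlay it binds OnEquipped to the equipped dispatcher.
; That handler scales BaseHealthRegen up and sets HealthRegen to a fixed value in the character's Stats struct, then calls AddXp with zero, apparently to refresh the stats.
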(event `self.ReceiveBeginPlay`
  (add `self.EquippedDispatcher` (delegate `On Equipped`))
  (`parent.ReceiveBeginPlay`))

(event `On Equipped` :!signature `self.EquippedDispatcher`
  (params (Character :type "MegadethCharacter Object Reference"))
  (bind _stats (`MegadethCharacter.Stats` Character))
  (bind _structout (setmembers `MegadethPlayerStats` :`StructRef` _stats :`BaseHealthRegen` (* (`.BaseHealthRegen` (break `MegadethPlayerStats` _stats)) 1.1) :`HealthRegen` 5.0))
  (set `MegadethCharacter.Stats` _structout Character)
  (`MegadethCharacter.AddXp` Character 0))