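; Pickup actor that grants an upgrade to a MegadethCharacter on overlap.
; On BeginPlay it creates a dynamic material on its Sphere and sets the texture to the SplashArt from the UpgradeToAdd class defaults.
; When a MegadethCharacter overlaps it, it adds UpgradeToAdd to that character as a component and destroys itself.
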(event `self.ReceiveBeginPlay`
  (bind _returnvalue (`PrimitiveComponent.CreateDynamicMaterialInstance` (`self.Sphere`) 0 "/Game/NewMaterial.NewMaterial" "None"))
  (`MaterialInstanceDynamic.SetTextureParameterValue` _returnvalue "Texture" (`.SplashArt` (defaults `Object` (`self.UpgradeToAdd`)))))

(event `self.ReceiveActorBeginOverlap`
  (params (OtherActor :type "Actor Object Reference"))
  (bind _asmegadeth_character (cast `MegadethCharacter` OtherActor))
  (bind _output_get (set `self.PlayerMegadethCharacter` _asmegadeth_character))
  (`|AddComponentByClass` _output_get (`self.UpgradeToAdd`))
  (`self.K2_DestroyActor`))

(fn `UserConstructionScript`)