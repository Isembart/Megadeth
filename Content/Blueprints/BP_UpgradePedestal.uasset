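; BP_UpgradePedestal is an interactable pedestal that offers a random upgrade and spawns it as a pickup.
; On BeginPlay it binds the interact event, picks a random upgrade from SkillsDataTable and shows Cost on its text component.
; A dynamic material instance puts the upgrade class's default SplashArt on the sphere.
; Interacting spawns a BP_UpgradePickup carrying that upgrade at an offset, with no cost check in this graph.
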(event `self.ReceiveBeginPlay`
  (`parent.ReceiveBeginPlay`)
  (add `self.InteractDelegate` (delegate `interactEvent`))
  (bind _outrownames (`DataTableFunctionLibrary.GetDataTableRowNames` (`self.SkillsDataTable`)))
  (bind _returnvalue (`|GetDataTableRow` (`self.SkillsDataTable`) (`KismetArrayLibrary.Array_Random` _outrownames))
    (:`then`
      (set `self.UpgradeToAdd` (`.Upgrade_4_249BC6254C4F60D313D42F80509374D4` (break `/Game/Structs/F_UpgradeRoulletteList` _returnvalue)))
      (`TextRenderComponent.K2_SetText` (`self.SkillName`) (`KismetTextLibrary.Conv_IntToText` (`self.Cost`)))
      (bind _returnvalue_2 (`PrimitiveComponent.CreateDynamicMaterialInstance` (`self.Sphere`) 0 "/Game/M_PickupOrbMaterial.M_PickupOrbMaterial" "None"))
      (`MaterialInstanceDynamic.SetTextureParameterValue` _returnvalue_2 "Texture" (`.SplashArt` (defaults `Object` (`self.UpgradeToAdd`)))))
    (:`RowNotFound`
      (`KismetSystemLibrary.PrintString` "BP_SkillPedestal ddn't find suitable skill in it's data table!"))))

(event `interactEvent` :!signature `self.InteractDelegate`
  (params (`Character To Interact` :type "MegadethCharacter Object Reference"))
  (`self.OnInteracted` `Character To Interact`))

(fn `OnInteracted`
  (params (Character :type "MegadethCharacter Object Reference"))
  (bind _returnvalue_location (`KismetMathLibrary.BreakTransform` (`self.GetTransform`)))
  (`|SpawnActorFromClass` "/Game/Blueprints/BP_UpgradePickup.BP_UpgradePickup_C" (`KismetMathLibrary.MakeTransform` (+ _returnvalue_location (-100.0 100.0 0.0))) "Undefined" "MultiplyWithRoot" null (`self.UpgradeToAdd`) null))

(fn `UserConstructionScript`)