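; Stage director that populates stages and handles stage/tavern transitions through MegadethStageSubsystem events.
; Entering a stage updates difficulty, spends a credit budget on upgrade pedestals with random data-table upgrades, spawns a teleporter and starts music.
; Placement uses random navmesh points that avoid the XY origin, with separate nav data for pedestals and teleporter; the teleporter retries until placed.
; Entering the tavern updates difficulty, stops music and gives the tavern portal a random level destination.
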(event `self.ReceiveBeginPlay`
  (bind _returnvalue (subsystem `MegadethStageSubsystem`))
  (`|ExecutionSequence`
    (:`then_0`
      (add `MegadethStageSubsystem.EnteredStage` _returnvalue (delegate `EnteredStage`))
      (bind _outactors (`GameplayStatics.GetAllActorsOfClass` "/Script/NavigationSystem.RecastNavMesh"))
      (`KismetSystemLibrary.PrintString` (`KismetStringLibrary.Conv_IntToString` (`KismetArrayLibrary.Array_Length` _outactors)))
      (`self.EnteredStage`))
    (:`then_1`
      (add `MegadethStageSubsystem.EnteredTavern` _returnvalue (delegate `EnteredTavern`)))))

(event `EnteredStage`
  (bind _output (`|ConvertAsset` (`self.InteractableTable`)))
  (`self.UpdateDifficulty`)
  (while (> (`self.InteractableCredits`) 0.0)
    (bind _outactors (`GameplayStatics.GetAllActorsOfClass` "/Script/NavigationSystem.RecastNavMesh"))
    (bind (_randomlocation _returnvalue) (`NavigationSystemV1.K2_GetRandomReachablePointInRadius` (`KismetMathLibrary.Vector_Zero`) (`self.LevelRadius`) (`|GetArrayItem` _outactors) null))
    (if (and _returnvalue (!= _randomlocation (`KismetMathLibrary.MakeVector` 0.0 0.0 (.z _randomlocation)) :`ErrorTolerance` 0.5))
      (bind _returnvalue_2 (`|SpawnActorFromClass` (`self.InteractableClass`) (`KismetMathLibrary.MakeTransform` _randomlocation) "Undefined" "MultiplyWithRoot" null null))
      (bind _asbp_upgrade_pedestal (cast `/Game/Blueprints/BP_UpgradePedestal` _returnvalue_2))
      (set `Actor.Tags` (`|MakeArray` "FieldUpgradePickup") _asbp_upgrade_pedestal)
      (set `self.InteractableCredits` (- (`self.InteractableCredits`) (`self.InteractableCost`)))
      (bind _outrownames (`DataTableFunctionLibrary.GetDataTableRowNames` _output))
      (bind _returnvalue_3 (`|GetDataTableRow` _output (`KismetArrayLibrary.Array_Random` _outrownames))
        (:`then`
          (set `/Game/Blueprints/BP_UpgradePedestal.UpgradeToAdd` (`.Upgrade_4_249BC6254C4F60D313D42F80509374D4` (break `/Game/Structs/F_UpgradeRoulletteList` _returnvalue_3)) _asbp_upgrade_pedestal)))))
  (bind _outactors_2 (`GameplayStatics.GetAllActorsOfClass` "/Script/NavigationSystem.RecastNavMesh"))
  (bind (_randomlocation_2 _returnvalue_4) (`NavigationSystemV1.K2_GetRandomLocationInNavigableRadius` (`KismetMathLibrary.Vector_Zero`) (`self.LevelRadius`) (`|GetArrayItem` _outactors_2 1) null :!label _label))
  (if (and _returnvalue_4 (!= _randomlocation_2 (`KismetMathLibrary.MakeVector` 0.0 0.0 (.z _randomlocation_2)) :`ErrorTolerance` 0.5))
    (`|SpawnActorFromClass` (`self.TeleporterClass`) (`KismetMathLibrary.MakeTransform` _randomlocation_2) "Undefined" "MultiplyWithRoot" null null)
    (`|ExecutionSequence`
      (:`then_0`
        (bind _outactors_3 (`GameplayStatics.GetAllActorsOfClassWithTag` "/Script/Engine.AmbientSound" "Music"))
        (`AudioComponent.Play` (`AmbientSound.AudioComponent` (`|GetArrayItem` _outactors_3)) 0.0))
      (:`then_1`
        (bind _outactors_4 (`GameplayStatics.GetAllActorsOfClassWithTag` "/Script/Engine.AmbientSound" "MusicTeleport"))
        (`AudioComponent.Stop` (`AmbientSound.AudioComponent` (`|GetArrayItem` _outactors_4)))))
    (else
      (`KismetSystemLibrary.PrintString` "Teleporter not spawned" true true (struct :`G` 0.66 :`B` 1.0 :`A` 1.0) 5.0)
      (goto _label))))

(event `EnteredTavern`
  (`self.UpdateDifficulty`)
  (bind _outactors (`GameplayStatics.GetAllActorsOfClassWithTag` "/Script/Engine.AmbientSound" "Music"))
  (`AudioComponent.Stop` (`AmbientSound.AudioComponent` (`|GetArrayItem` _outactors)))
  (bind _randomlocation (`NavigationSystemV1.K2_GetRandomLocationInNavigableRadius` (`KismetMathLibrary.Vector_Zero`) 10000.0 null null))
  (bind _outactors_2 (`GameplayStatics.GetAllActorsWithTag` "TavernPortal"))
  (bind _asbp_tavern_portal (cast `/Game/Blueprints/BP_TavernPortal` (`|GetArrayItem` _outactors_2)))
  (set `/Game/Blueprints/BP_TavernPortal.LevelLocation` _randomlocation _asbp_tavern_portal))

(fn `UserConstructionScript`)