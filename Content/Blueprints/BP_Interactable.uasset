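; BP_Interactable is an interactable that costs gold, with its cost scaled at BeginPlay by the difficulty coefficient raised to a power.
; Overlap by a MegadethCharacter with enough gold shows a prompt widget and enables input; leaving hides and disables them.
; Completing IA_Interact disables further interaction, then rechecks gold before deducting it and calling the interact delegate.
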(event `self.InteractCollision.OnComponentBeginOverlap`
  (params (OverlappedComponent :type "PrimitiveComponent Object Reference") (OtherActor :type "Actor Object Reference") (OtherComp :type "PrimitiveComponent Object Reference") (OtherBodyIndex :type Integer) (bFromSweep :type Boolean) (SweepResult :type "HitResult Structure (by ref)"))
  (if (`self.enabled`)
    (bind _asmegadeth_character (cast `MegadethCharacter` OtherActor))
    (bind _output_get (set `self.MegadethCharacter` _asmegadeth_character))
    (if (>= (`.Gold` (break `MegadethPlayerStats` (`MegadethCharacter.Stats` _output_get))) (`self.Cost`))
      (`Widget.SetVisibility` (`WidgetComponent.GetWidget` (`self.InteractNotify`)) "Visible")
      (set `self.canInteract` true)
      (`self.EnableInput` (`GameplayStatics.GetPlayerController` 0)))))

(event `self.ReceiveBeginPlay`
  (`Widget.SetVisibility` (`WidgetComponent.GetWidget` (`self.InteractNotify`)) "Hidden")
  (set `self.Cost` (`KismetMathLibrary.FTrunc` (* (`self.Cost`) (`KismetMathLibrary.MultiplyMultiply_FloatFloat` (`MegadethDifficultySubsystem.DifficultyCoefficient` (subsystem `MegadethDifficultySubsystem`)) 1.25)))))

(event `self.InteractCollision.OnComponentEndOverlap`
  (params (OverlappedComponent :type "PrimitiveComponent Object Reference") (OtherActor :type "Actor Object Reference") (OtherComp :type "PrimitiveComponent Object Reference") (OtherBodyIndex :type Integer))
  (bind _returnvalue (`WidgetComponent.GetWidget` (`self.InteractNotify`)))
  (cast `MegadethCharacter` OtherActor)
  (`/Engine/EditorBlueprintResources/StandardMacros.IsValid` _returnvalue
    (:`Is Valid`
      (`Widget.SetVisibility` _returnvalue "Hidden")
      (set `self.canInteract` false)
      (`self.DisableInput` (`GameplayStatics.GetPlayerController` 0)))))

(event `EnhancedInput|/Game/TopDown/Input/Actions/IA_Interact`
  (params (ActionValue :type Boolean) (ElapsedSeconds :type "Float (double-precision)") (TriggeredSeconds :type "Float (double-precision)") (InputAction :type "InputAction Object Reference" :default "/Game/TopDown/Input/Actions/IA_Interact.IA_Interact"))
  (bind _megadethcharacter (`self.MegadethCharacter`))
  (bind _cost (`self.Cost`))
  (:`Completed`
    (if (and (`self.enabled`) (`self.canInteract`))
      (`/Engine/EditorBlueprintResources/StandardMacros.IsValid` _megadethcharacter
        (:`Is Valid`
          (`self.CompleteInteraction`)
          (if (>= (`.Gold` (break `MegadethPlayerStats` (`MegadethCharacter.Stats` _megadethcharacter))) _cost)
            (`MegadethCharacter.AddGold` _megadethcharacter (* _cost -1))
            (`self.InteractDelegate` _megadethcharacter)))))))

(fn `CompleteInteraction`
  (set `self.enabled` false)
  (`Widget.SetVisibility` (`WidgetComponent.GetWidget` (`self.InteractNotify`)) "Hidden"))

(fn `UserConstructionScript`)