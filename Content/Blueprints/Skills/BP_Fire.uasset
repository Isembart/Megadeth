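; BP_Fire is a skill actor that creates a fire area, damaging enemies inside it over six seconds before destroying itself.
; On spawn it caches the player character's crit chance and starts a self-repeating tick every half second.
; Each tick queries actors overlapping its sphere collision and damages each BP_Enemy, rolling per hit for a double-damage crit flagged with a crit damage type.
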(event `self.ReceiveBeginPlay`
  (bind _asmegadeth_character (cast `MegadethCharacter` (`GameplayStatics.GetPlayerPawn` 0)))
  (set `self.Crit Chance` (`.CritChance` (break `MegadethPlayerStats` (`MegadethCharacter.Stats` _asmegadeth_character))))
  (`self.FireTick`)
  (`KismetSystemLibrary.Delay` 6.0)
  (`self.K2_DestroyActor`))

(event `FireTick`
  (bind _spherecollision (`self.SphereCollision`))
  (bind _damage (`self.Damage`))
  (bind _outactors (`KismetSystemLibrary.ComponentOverlapActors` _spherecollision (`SceneComponent.K2_GetComponentToWorld` _spherecollision) (`self.Object Types`)))
  (for _array_element _outactors
    (bind _asbp_enemy (cast `/Game/Blueprints/Enemies/BP_Enemy` _array_element))
    (if (< (`KismetMathLibrary.RandomFloatInRange` 0.0 100.0) (`self.Crit Chance`))
      (`GameplayStatics.ApplyDamage` _asbp_enemy (* _damage 2.0) null null "/Game/Blueprints/BP_DamageTypeCrit.BP_DamageTypeCrit_C")
      (else
        (`GameplayStatics.ApplyDamage` _asbp_enemy _damage))))
  (`KismetSystemLibrary.Delay` 0.5)
  (`self.FireTick`))

(fn `UserConstructionScript`)