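; BP_Dash is a skill actor that makes a character dash horizontally along its forward direction.
; InvokeAbility stops the character's movement, disables player 0's input and switches movement to walking.
; A Dash timeline then overrides velocity each update, scaling the forward vector by its DistanceMultiplier track and a fixed speed, with vertical velocity zeroed.
; When the timeline finishes, input is re-enabled and the actor destroys itself.
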(event `self.ReceiveBeginPlay`)

(event `self.InvokeAbility`
  (params (Character :type "MegadethCharacter Object Reference") (Damage :type Integer))
  (bind _returnvalue (`GameplayStatics.GetPlayerController` 0))
  (bind _returnvalue_2 (`GameplayStatics.GetPlayerController` 0))
  (bind _character (`self.Character`))
  (bind _output_get (set `self.Character` Character))
  (`MovementComponent.StopMovementImmediately` (`Character.CharacterMovement` _output_get))
  (`self.DisableInput` _returnvalue_2 _returnvalue_2)
  (`CharacterMovementComponent.SetMovementMode` (`Character.CharacterMovement` (`self.Character`)) "MOVE_Walking" 0)
  (bind (_direction _distancemultiplier) (`Timeline|Dash` :!via `PlayFromStart`)
    (:`Update`
      (bind (_returnvalue_x _returnvalue_y) (`KismetMathLibrary.BreakVector` (* (`SceneComponent.GetForwardVector` (`Actor.RootComponent` _character)) (* _distancemultiplier 4000.0))))
      (set `MovementComponent.Velocity` (`KismetMathLibrary.MakeVector` _returnvalue_x _returnvalue_y) (`Character.CharacterMovement` _character)))
    (:`Finished`
      (`self.EnableInput` _returnvalue _returnvalue)
      (`self.K2_DestroyActor`))))

(fn `UserConstructionScript`)