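; BP_PlayerMine is a player skill mine that explodes when a BP_Enemy enters its ActivationSphere.
; The explosion plays an energy orb sound and applies radial damage with distance falloff, ignoring the mine itself.
; Two chained timelines then scale the TPBubble, the first played forward and the second in reverse, before the actor destroys itself.
; The DamageSphere overlap event is empty.
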(event `Explode`
  (bind _returnvalue (`self.K2_GetActorLocation`))
  (`GameplayStatics.PlaySoundAtLocation` "/Game/Audio/SCIEnrg_Energy_Orb_05.SCIEnrg_Energy_Orb_05" _returnvalue (struct) 1.0 1.0 0.0 null null null null)
  (`GameplayStatics.ApplyRadialDamageWithFalloff` (`self.Damage`) 10.0 _returnvalue 200.0 300.0 2.0 "/Script/Engine.DamageType" (`|MakeArray` self) null null)
  (bind (_direction _bubblesize) (`Timeline|ExplodeRadius` :!via `PlayFromStart`)
    (:`Update`
      (`SceneComponent.SetRelativeScale3D` (`self.TPBubble`) (`KismetMathLibrary.Conv_DoubleToVector` _bubblesize)))
    (:`Finished`
      (bind (_direction_2 _bubblesize_2) (`Timeline|Oś czasu` :!via `ReverseFromEnd`)
        (:`Update`
          (`SceneComponent.SetRelativeScale3D` (`self.TPBubble`) (`KismetMathLibrary.Conv_DoubleToVector` _bubblesize_2)))
        (:`Finished`
          (`self.K2_DestroyActor`))))))

(event `self.ActivationSphere.OnComponentBeginOverlap`
  (params (OverlappedComponent :type "PrimitiveComponent Object Reference") (OtherActor :type "Actor Object Reference") (OtherComp :type "PrimitiveComponent Object Reference") (OtherBodyIndex :type Integer) (bFromSweep :type Boolean) (SweepResult :type "HitResult Structure (by ref)"))
  (cast `/Game/Blueprints/Enemies/BP_Enemy` OtherActor)
  (`self.Explode`))

(event `self.DamageSphere.OnComponentBeginOverlap`
  (params (OverlappedComponent :type "PrimitiveComponent Object Reference") (OtherActor :type "Actor Object Reference") (OtherComp :type "PrimitiveComponent Object Reference") (OtherBodyIndex :type Integer) (bFromSweep :type Boolean) (SweepResult :type "HitResult Structure (by ref)")))

(fn `UserConstructionScript`)