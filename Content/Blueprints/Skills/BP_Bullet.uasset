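; BP_Bullet is a projectile that damages BP_Enemy actors it overlaps, using a separate damage type for critical shots.
; Tick moves it forward at constant speed with a swept offset, then calls StickTOGround.
; That step traces downward, ignoring the player pawn, and holds the bullet at a fixed height above nearby ground so it follows terrain.
; It destroys itself on enemy overlap, on any hit, or when its short lifetime expires.
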(event `self.ReceiveBeginPlay`
  (`KismetSystemLibrary.Delay` 5.0)
  (`self.K2_DestroyActor`))

(event `self.ReceiveTick`
  (params (DeltaSeconds :type "Float (single-precision)"))
  (bind (_returnvalue_x _returnvalue_y) (`KismetMathLibrary.BreakVector` (`self.K2_GetActorLocation`)))
  (bind _returnvalue (`self.K2_GetActorLocation`))
  (`self.K2_AddActorWorldOffset` (* (`self.GetActorForwardVector`) (`KismetMathLibrary.Conv_DoubleToVector` 5000.0) DeltaSeconds) true)
  (bind (_outhit _returnvalue_2) (`KismetSystemLibrary.LineTraceSingle` _returnvalue (- _returnvalue (0.0 0.0 1000.0)) "TraceTypeQuery1" false (`|MakeArray` (`GameplayStatics.GetPlayerPawn` 0) :!type "Actor Object Reference")))
  (bind _z (.z (`.Location` (`GameplayStatics.BreakHitResult` _outhit))))
  (if (and (< (- (.z _returnvalue) _z) 200.0) _returnvalue_2)
    (`self.K2_SetActorLocation` (`KismetMathLibrary.MakeVector` _returnvalue_x _returnvalue_y (+ _z 100.0)))))

(event `self.ReceiveActorBeginOverlap`
  (params (OtherActor :type "Actor Object Reference"))
  (bind _damage (`self.Damage`))
  (bind _asbp_enemy (cast `/Game/Blueprints/Enemies/BP_Enemy` OtherActor))
  (if (`self.isCritical`)
    (`GameplayStatics.ApplyDamage` _asbp_enemy _damage null null "/Game/Blueprints/BP_DamageTypeCrit.BP_DamageTypeCrit_C")
    (else
      (`GameplayStatics.ApplyDamage` _asbp_enemy _damage)))
  (`self.K2_DestroyActor`))

(event `self.ReceiveHit`
  (params (MyComp :type "PrimitiveComponent Object Reference") (Other :type "Actor Object Reference") (OtherComp :type "PrimitiveComponent Object Reference") (bSelfMoved :type Boolean) (HitLocation :type "Vector Structure") (HitNormal :type "Vector Structure") (NormalImpulse :type "Vector Structure") (Hit :type "HitResult Structure (by ref)"))
  (`self.K2_DestroyActor`))

(fn `UserConstructionScript`)