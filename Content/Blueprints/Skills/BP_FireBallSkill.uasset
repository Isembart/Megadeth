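; BP_FireBallSkill is a short-lived skill actor that casts a fireball from the invoking character.
; InvokeAbility halts and disables the character's movement, then spawns a BP_FireBallBullet using the character's location and rotation.
; The bullet receives the passed damage multiplied by AbilityData.AbilityDamage and has overlap events enabled on its sphere collision.
; After a brief delay, walking is restored and the skill actor destroys itself.
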(event `self.InvokeAbility`
  (params (Character :type "MegadethCharacter Object Reference") (Damage :type Integer))
  (bind (_returnvalue_location _returnvalue_rotation) (`KismetMathLibrary.BreakTransform` (`self.GetTransform` Character)))
  (bind _charactermovement (`Character.CharacterMovement` Character))
  (bind (_abilitydata_abilityname _abilitydata_abilitycooldown _abilitydata_abilitydamage) (break `MegadethAbilityData` (`self.AbilityData`)))
  (`MovementComponent.StopMovementImmediately` _charactermovement)
  (`CharacterMovementComponent.DisableMovement` _charactermovement)
  (`WidgetLayoutLibrary.GetMousePositionOnViewport`)
  (bind _returnvalue (`|SpawnActorFromClass` "/Game/Blueprints/BP_FireBallBullet.BP_FireBallBullet_C" (`KismetMathLibrary.MakeTransform` (+ _returnvalue_location (* (`self.GetActorForwardVector` Character) (`KismetMathLibrary.Conv_DoubleToVector` 0.0))) _returnvalue_rotation) "Undefined" "MultiplyWithRoot" null (* Damage _abilitydata_abilitydamage) null))
  (set `PrimitiveComponent.bGenerateOverlapEvents` true (`/Game/Blueprints/BP_FireBallBullet.SphereCollision` _returnvalue))
  (`KismetSystemLibrary.Delay` 0.2)
  (`CharacterMovementComponent.SetMovementMode` _charactermovement "MOVE_Walking" 0)
  (`self.K2_DestroyActor`))

(fn `UserConstructionScript`)