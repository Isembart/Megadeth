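; BP_KillerBullet is a skill actor that fires a BP_KillerBulletBullet projectile when its ability is invoked.
; InvokeAbility spawns the projectile at the character's location and rotation, passing the crit flag and incoming damage scaled by the ability's damage value.
; It plays a silenced pistol sound in 2D, then destroys itself after a short delay.
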(event `self.InvokeAbility`
  (params (Character :type "MegadethCharacter Object Reference") (Damage :type Integer) (bIsCrit :type Boolean))
  (bind (_returnvalue_location _returnvalue_rotation) (`KismetMathLibrary.BreakTransform` (`self.GetTransform` Character)))
  (bind (_abilitydata_abilityname _abilitydata_abilitycooldown _abilitydata_abilitydamage) (break `MegadethAbilityData` (`self.AbilityData`)))
  (`|SpawnActorFromClass` "/Game/Blueprints/Skills/BP_KillerBulletBullet.BP_KillerBulletBullet_C" (`KismetMathLibrary.MakeTransform` (+ _returnvalue_location (* (`self.GetActorForwardVector` Character) (`KismetMathLibrary.Conv_DoubleToVector` 0.0))) _returnvalue_rotation) "Undefined" "MultiplyWithRoot" null (* Damage _abilitydata_abilitydamage) bIsCrit null)
  (`GameplayStatics.PlaySound2D` "/Game/Audio/GUNSupr_Silenced_Pistol_Fire_Short_01.GUNSupr_Silenced_Pistol_Fire_Short_01" 1.0 1.0 0.0 null null)
  (`KismetSystemLibrary.Delay` 0.2)
  (`self.K2_DestroyActor`))

(fn `UserConstructionScript`)