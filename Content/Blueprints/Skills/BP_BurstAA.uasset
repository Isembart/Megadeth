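; Burst auto-attack skill actor that fires five quick shots from the invoking character, then destroys itself.
; InvokeAbility runs five duplicated Shoot graphs separated by short delays, passing damage scaled by AbilityData.AbilityDamage and the crit flag.
; Each shot spawns a BP_Bullet at the character's current transform with a zero forward offset and plays a silenced pistol sound.
; Shoot_3 is the exception, as its spawn node has no class set.
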(event `self.InvokeAbility`
  (params (Character :type "MegadethCharacter Object Reference") (Damage :type Integer) (bIsCrit :type Boolean))
  (bind (_returnvalue_location _returnvalue_rotation) (`KismetMathLibrary.BreakTransform` (`self.GetTransform` Character)))
  (bind (_returnvalue_location_2 _returnvalue_rotation_2) (`KismetMathLibrary.BreakTransform` (`self.GetTransform` Character)))
  (bind (_returnvalue_location_3 _returnvalue_rotation_3) (`KismetMathLibrary.BreakTransform` (`self.GetTransform` Character)))
  (bind (_returnvalue_location_4 _returnvalue_rotation_4) (`KismetMathLibrary.BreakTransform` (`self.GetTransform` Character)))
  (bind (_returnvalue_location_5 _returnvalue_rotation_5) (`KismetMathLibrary.BreakTransform` (`self.GetTransform` Character)))
  (bind (_abilitydata_abilityname _abilitydata_abilitycooldown _abilitydata_abilitydamage) (break `MegadethAbilityData` (`self.AbilityData`)))
  (`|SpawnActorFromClass` "/Game/Blueprints/Skills/BP_Bullet.BP_Bullet_C" (`KismetMathLibrary.MakeTransform` (+ _returnvalue_location_2 (* (`self.GetActorForwardVector` Character) (`KismetMathLibrary.Conv_DoubleToVector` 0.0))) _returnvalue_rotation_2) "Undefined" "MultiplyWithRoot" null (* Damage _abilitydata_abilitydamage) bIsCrit null)
  (`GameplayStatics.PlaySound2D` "/Game/Audio/GUNSupr_Silenced_Pistol_Fire_Short_01.GUNSupr_Silenced_Pistol_Fire_Short_01" 1.0 1.0 0.0 null null)
  (`KismetSystemLibrary.Delay` 0.08)
  (`|SpawnActorFromClass` "/Game/Blueprints/Skills/BP_Bullet.BP_Bullet_C" (`KismetMathLibrary.MakeTransform` (+ _returnvalue_location_3 (* (`self.GetActorForwardVector` Character) (`KismetMathLibrary.Conv_DoubleToVector` 0.0))) _returnvalue_rotation_3) "Undefined" "MultiplyWithRoot" null (* Damage _abilitydata_abilitydamage) bIsCrit null)
  (`GameplayStatics.PlaySound2D` "/Game/Audio/GUNSupr_Silenced_Pistol_Fire_Short_01.GUNSupr_Silenced_Pistol_Fire_Short_01" 1.0 1.0 0.0 null null)
  (`KismetSystemLibrary.Delay` 0.08)
  (`|SpawnActorFromClass` "/Game/Blueprints/Skills/BP_Bullet.BP_Bullet_C" (`KismetMathLibrary.MakeTransform` (+ _returnvalue_location_4 (* (`self.GetActorForwardVector` Character) (`KismetMathLibrary.Conv_DoubleToVector` 0.0))) _returnvalue_rotation_4) "Undefined" "MultiplyWithRoot" null (* Damage _abilitydata_abilitydamage) bIsCrit null)
  (`GameplayStatics.PlaySound2D` "/Game/Audio/GUNSupr_Silenced_Pistol_Fire_Short_01.GUNSupr_Silenced_Pistol_Fire_Short_01" 1.0 1.0 0.0 null null)
  (`KismetSystemLibrary.Delay` 0.08)
  (`|SpawnActorFromClass` "/Game/Blueprints/Skills/BP_Bullet.BP_Bullet_C" (`KismetMathLibrary.MakeTransform` (+ _returnvalue_location_5 (* (`self.GetActorForwardVector` Character) (`KismetMathLibrary.Conv_DoubleToVector` 0.0))) _returnvalue_rotation_5) "Undefined" "MultiplyWithRoot" null (* Damage _abilitydata_abilitydamage) bIsCrit null)
  (`GameplayStatics.PlaySound2D` "/Game/Audio/GUNSupr_Silenced_Pistol_Fire_Short_01.GUNSupr_Silenced_Pistol_Fire_Short_01" 1.0 1.0 0.0 null null)
  (`KismetSystemLibrary.Delay` 0.08)
  (`|SpawnActorFromClass` "/Game/Blueprints/Skills/BP_Bullet.BP_Bullet_C" (`KismetMathLibrary.MakeTransform` (+ _returnvalue_location (* (`self.GetActorForwardVector` Character) (`KismetMathLibrary.Conv_DoubleToVector` 0.0))) _returnvalue_rotation) "Undefined" "MultiplyWithRoot" null (* Damage _abilitydata_abilitydamage) bIsCrit null)
  (`GameplayStatics.PlaySound2D` "/Game/Audio/GUNSupr_Silenced_Pistol_Fire_Short_01.GUNSupr_Silenced_Pistol_Fire_Short_01" 1.0 1.0 0.0 null null)
  (`KismetSystemLibrary.Delay` 0.08)
  (`self.K2_DestroyActor`))

(fn `UserConstructionScript`)