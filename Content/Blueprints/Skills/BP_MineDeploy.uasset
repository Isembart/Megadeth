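; BP_MineDeploy is a skill actor that places a player mine on the ground beneath the character using it.
; When invoked, it line-traces straight down from the character, ignoring that character, and spawns BP_PlayerMine at the hit location.
; The mine's damage is the passed-in damage scaled by the ability data's damage value.
; It then plays a deploy sound and destroys itself, acting as a one-shot ability.
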(event `self.ReceiveBeginPlay`)

(event `self.InvokeAbility`
  (params (Character :type "MegadethCharacter Object Reference") (Damage :type Integer) (bIsCrit :type Boolean))
  (bind _returnvalue (`self.K2_GetActorLocation` Character))
  (bind (_abilitydata_abilityname _abilitydata_abilitycooldown _abilitydata_abilitydamage) (break `MegadethAbilityData` (`self.AbilityData`)))
  (bind _outhit (`KismetSystemLibrary.LineTraceSingle` _returnvalue (- _returnvalue (0.0 0.0 300.0)) "TraceTypeQuery1" false (`|MakeArray` Character)))
  (`|SpawnActorFromClass` "/Game/Blueprints/Skills/BP_PlayerMine.BP_PlayerMine_C" (`KismetMathLibrary.MakeTransform` (`.Location` (`GameplayStatics.BreakHitResult` _outhit))) "Undefined" "MultiplyWithRoot" null (* (`KismetMathLibrary.Conv_IntToDouble` Damage) _abilitydata_abilitydamage) null)
  (`GameplayStatics.PlaySound2D` "/Game/Audio/MECHClik_Mine_Deploy_02.MECHClik_Mine_Deploy_02" 1.0 1.0 0.0 null null)
  (`self.K2_DestroyActor`))

(fn `UserConstructionScript`)