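; Enemy Blueprint that fires bullets at the player through a Shoot event.
; After a short delay, Shoot turns the enemy on yaw toward the player pawn, spawns a BP_ENEMYBullet just in front of it with its Damage value and plays a silenced pistol sound in 2D.
; BeginPlay, overlap and Tick are disabled stubs, and nothing in this file calls or repeats Shoot.
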(event `Shoot`
  (bind (_returnvalue_location _returnvalue_rotation) (`KismetMathLibrary.BreakTransform` (`self.GetTransform`)))
  (bind (_returnvalue_roll _returnvalue_pitch _returnvalue_yaw) (`KismetMathLibrary.BreakRotator` (`KismetMathLibrary.FindLookAtRotation` (`self.K2_GetActorLocation`) (`self.K2_GetActorLocation` (`GameplayStatics.GetPlayerPawn` 0)))))
  (`KismetSystemLibrary.Delay` 1.0)
  (`self.K2_SetActorRotation` (`KismetMathLibrary.MakeRotator` 0.0 0.0 _returnvalue_yaw))
  (`|SpawnActorFromClass` "/Game/Blueprints/Skills/BP_ENEMYBullet.BP_ENEMYBullet_C" (`KismetMathLibrary.MakeTransform` (+ _returnvalue_location (* (`self.GetActorForwardVector`) (`KismetMathLibrary.Conv_DoubleToVector` 10.0))) _returnvalue_rotation) "Undefined" "MultiplyWithRoot" null (`self.Damage`) false null)
  (`GameplayStatics.PlaySound2D` "/Game/Audio/GUNSupr_Silenced_Pistol_Fire_Short_01.GUNSupr_Silenced_Pistol_Fire_Short_01" 1.0 1.0 0.0 null null))

(fn `UserConstructionScript`
  (`parent.UserConstructionScript`))