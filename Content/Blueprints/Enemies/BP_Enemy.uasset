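; BP_Enemy is an enemy that deals contact damage to the player and shows feedback when it is hit.
; While a MegadethCharacter overlaps it, Tick counts down a timer and applies damage to the player at each interval.
; Taking damage refreshes the widget health bar, spawns a randomly offset popup flagged for crits by damage type class, and plays a hit-marker sound.
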(event `self.ReceiveTick`
  (params (DeltaSeconds :type "Float (single-precision)"))
  (`parent.ReceiveTick` DeltaSeconds)
  (if (`self.Damaging`)
    (set `self.RemainingTimeToDamage` (- (`self.RemainingTimeToDamage`) DeltaSeconds))
    (if (<= (`self.RemainingTimeToDamage`) 0.0)
      (set `self.RemainingTimeToDamage` (`self.TimeToDamage`))
      (`GameplayStatics.ApplyDamage` (`self.Player`) (`self.Damage`)))))

(event `self.ReceiveActorEndOverlap`
  (params (OtherActor :type "Actor Object Reference"))
  (cast `MegadethCharacter` OtherActor)
  (set `self.Damaging` false))

(event `self.ReceiveActorBeginOverlap`
  (params (OtherActor :type "Actor Object Reference"))
  (cast `MegadethCharacter` OtherActor)
  (set `self.Damaging` true))

(event `self.ReceiveAnyDamage`
  (params (Damage :type "Float (single-precision)") (DamageType :type "DamageType Object Reference") (InstigatedBy :type "Controller Object Reference") (DamageCauser :type "Actor Object Reference"))
  (`self.UpdateHealthBar`)
  (bind _returnvalue (`|SpawnActorFromClass` "/Game/Blueprints/BP_DamagePopUpActor.BP_DamagePopUpActor_C" (`KismetMathLibrary.MakeTransform` (+ (`self.K2_GetActorLocation`) (`KismetMathLibrary.MakeVector` (`KismetMathLibrary.RandomFloatInRange` -40.0 40.0) (`KismetMathLibrary.RandomFloatInRange` -40.0 40.0) (`KismetMathLibrary.RandomFloatInRange` 40.0 80.0)))) "Undefined" "MultiplyWithRoot" null (== (`GameplayStatics.GetObjectClass` DamageType) "/Game/Blueprints/BP_DamageTypeCrit.BP_DamageTypeCrit_C") null))
  (`/Game/Blueprints/BP_DamagePopUpActor.ChangeText` _returnvalue (`KismetTextLibrary.Conv_DoubleToText` Damage "HalfToEven"))
  (`GameplayStatics.PlaySound2D` "/Game/Audio/BLLTImpt_Hit_Marker_07.BLLTImpt_Hit_Marker_07" 1.0 1.0 0.0 null null))

(event `self.ReceiveBeginPlay`
  (bind _asw_health_bar (cast `/Game/UI/W_HealthBar` (`WidgetComponent.GetWidget` (`self.Widget`))))
  (set `self.As W Health Bar` _asw_health_bar)
  (`self.UpdateHealthBar`))

(fn `UpdateHealthBar`
  (`/Game/UI/W_HealthBar.UpdateHealthBar` (`self.As W Health Bar`) (/ (`self.Health`) (`self.MaxHealth`))))

(fn `UserConstructionScript`)