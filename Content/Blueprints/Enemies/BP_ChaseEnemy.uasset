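; Enemy Blueprint that relentlessly chases the Player through AI movement, extending a parent class.
; BeginPlay starts a looping AI MoveTo with continuous goal tracking, polling briefly whenever the Player reference is invalid.
; A finished move restarts the chase, while a failed request first moves to a random nearby navigable point before retrying.
; Overlap, Tick and construction only call the parent.
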(event `self.ReceiveBeginPlay`
  (bind _player (`self.Player`))
  (`parent.ReceiveBeginPlay`)
  (`/Engine/EditorBlueprintResources/StandardMacros.IsValid` _player :!label _label
    (:`Is Valid`
      (`AITask_MoveTo.AIMoveTo` (`AIBlueprintHelperLibrary.GetAIController` self) (0.0 0.0 0.0) _player -1.0 "Disable" "Enable" true false true
        (:`OnRequestFailed`
          (bind _randomlocation (`NavigationSystemV1.K2_GetRandomLocationInNavigableRadius` (`self.K2_GetActorLocation`) 300.0 null null))
          (`|AIMoveTo` self _randomlocation null
            (:`OnSuccess`
              (goto _label))
            (:`OnFail`
              (goto _label))))
        (:`OnMoveFinished`
          (goto _label))))
    (:`Is Not Valid`
      (`KismetSystemLibrary.Delay` 0.1)
      (goto _label))))

(event `self.ReceiveActorBeginOverlap`
  (params (OtherActor :type "Actor Object Reference"))
  (`parent.ReceiveActorBeginOverlap` OtherActor))

(event `self.ReceiveTick`
  (params (DeltaSeconds :type "Float (single-precision)"))
  (`parent.ReceiveTick` DeltaSeconds))

(fn `UserConstructionScript`
  (`parent.UserConstructionScript`))