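; BP_PortalCarrier is a wandering enemy that leaves a tavern portal behind when it dies.
; On BeginPlay it starts roaming, repeatedly using AIMoveTo toward random navigable points around itself, re-picking only when a move succeeds.
; A handler bound to OnDeath spawns a BP_TavernPortal at the carrier's location and tags it FieldPortal.
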(event `self.ReceiveBeginPlay`
  (`parent.ReceiveBeginPlay`)
  (add `MegadethEnemy.OnDeath` (delegate `CustomEvent`))
  (`self.MoveToRandomLocation`))

(event `CustomEvent`
  (bind _returnvalue_location (`KismetMathLibrary.BreakTransform` (`self.GetTransform`)))
  (bind _returnvalue (`|SpawnActorFromClass` "/Game/Blueprints/BP_TavernPortal.BP_TavernPortal_C" (`KismetMathLibrary.MakeTransform` _returnvalue_location) "Undefined" "MultiplyWithRoot" null null))
  (set `Actor.Tags` (`|MakeArray` "FieldPortal") _returnvalue))

(event `MoveToRandomLocation`
  (bind _randomlocation (`NavigationSystemV1.K2_GetRandomLocationInNavigableRadius` (`self.K2_GetActorLocation`) 1000.0 null null))
  (`|AIMoveTo` self _randomlocation null 50.0
    (:`OnSuccess`
      (`self.MoveToRandomLocation`))))

(fn `UserConstructionScript`
  (`parent.UserConstructionScript`))